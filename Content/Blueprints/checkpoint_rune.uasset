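; A checkpoint rune actor that saves the player's progress on first touch.
; Overlap by the player character stores its location, health and shield energy on that character, plays a sound and activates the checkpoint effects.
; A CheckpointPassed flag prevents repeat saves.
; A Timeline started on BeginPlay moves the root vertically between its initial position and a raised one, while Tick spins it slowly around yaw.
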(event `self.checkpoint_collision.OnComponentBeginOverlap`
  (params (OverlappedComponent :type "PrimitiveComponent Object Reference") (OtherActor :type "Actor Object Reference") (OtherComp :type "PrimitiveComponent Object Reference") (OtherBodyIndex :type Integer) (bFromSweep :type Boolean) (SweepResult :type "HitResult Structure (by ref)"))
  (bind _player_reference (`self.player Reference`))
  ;[1 1 1] Save Player locaiton and health
  (if (== OtherActor (`self.player Reference`))
    (if (not (`self.checkpoint_passed`))
      (`|ExecutionSequence`
        (:`then_0`
          (`self.SetLastCheckpoint`)
          (`GameplayStatics.PlaySound2D` "/Game/SoundClips/checkpoint.checkpoint" 1.0 1.0 0.0 null null))
        (:`then_1`
          (set `/Game/ThirdPerson/Blueprints/BP_ThirdPersonCharacter.checkpoint_health` (`/Game/ThirdPerson/Blueprints/BP_ThirdPersonCharacter.Health` _player_reference) _player_reference))
        (:`then_2`
          (set `/Game/ThirdPerson/Blueprints/BP_ThirdPersonCharacter.checkpoint_shield` (`/Game/ThirdPerson/Blueprints/BP_ThirdPersonCharacter.shield_energy` _player_reference) _player_reference))
        (:`then_3`
          (set `self.checkpoint_passed` true)
          (`ActorComponent.Activate` (`self.checkpoint used`) false)
          (`ActorComponent.Activate` (`self.checkpoint effects`) false))))))

(event `SetLastCheckpoint`
  (bind _player_reference (`self.player Reference`))
  ;[1 1 1] Log Checkpoint Location
  (set `/Game/ThirdPerson/Blueprints/BP_ThirdPersonCharacter.lastCheckPoint` (`self.K2_GetActorLocation` _player_reference) _player_reference))

(event `self.ReceiveBeginPlay`
  (bind _asbp_third_person_character (cast `/Game/ThirdPerson/Blueprints/BP_ThirdPersonCharacter` (`GameplayStatics.GetPlayerCharacter` 0)))
  (set `self.player Reference` _asbp_third_person_character)
  (bind _output_get (set `self.InitialLocation` (`SceneComponent.RelativeLocation` (`self.DefaultSceneRoot`))))
  (bind (_direction _lerp) (`Timeline|Timeline` :!via `PlayFromStart`)
    (:`Update`
      (bind (_returnvalue_x _returnvalue_y _returnvalue_z) (`KismetMathLibrary.BreakVector` (`KismetMathLibrary.VLerp` (`KismetMathLibrary.MakeVector` (.x _output_get) (.y _output_get) (.z _output_get)) (`KismetMathLibrary.MakeVector` (.x _output_get) (.y _output_get) (+ (.z _output_get) 50.0)) _lerp)))
      (`SceneComponent.K2_SetWorldLocation` (`self.DefaultSceneRoot`) (`KismetMathLibrary.MakeVector` _returnvalue_x _returnvalue_y _returnvalue_z) false false))))

(event `self.ReceiveTick`
  (params (DeltaSeconds :type "Float (single-precision)"))
  (`SceneComponent.K2_AddLocalRotation` (`self.DefaultSceneRoot`) (`KismetMathLibrary.MakeRotator` 0.0 0.0 (* DeltaSeconds 20.0)) false false))

(fn `UserConstructionScript`)