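; Energy shield actor that blocks projectiles while active.
; Custom events switch it on and off by toggling the overlap component's collision profile and visibility along with the ShieldTexture effect.
; Any BP_Projectile that begins overlapping the shield is destroyed, and a 2D block sound plays.
; Activation also prints a leftover debug string.
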(event `self.shield_overlap.OnComponentBeginOverlap`
  (params (OverlappedComponent :type "PrimitiveComponent Object Reference") (OtherActor :type "Actor Object Reference") (OtherComp :type "PrimitiveComponent Object Reference") (OtherBodyIndex :type Integer) (bFromSweep :type Boolean) (SweepResult :type "HitResult Structure (by ref)"))
  ;[1 1 1] Destroy Projectile
  (bind _asbp_projectile (cast `/Game/Blueprints/BP_Projectile` OtherActor))
  (if (== OtherActor _asbp_projectile)
    (`self.K2_DestroyActor` OtherActor)
    (`GameplayStatics.PlaySound2D` "/Game/SoundClips/energyshieldblock_Cue.energyshieldblock_Cue" 1.0 1.0 0.0 null null)))

(event `shield_active`
  (bind _shield_overlap (`self.shield_overlap`))
  ;[1 1 1] Shield Logic
  (`PrimitiveComponent.SetCollisionProfileName` _shield_overlap "OverlapAllDynamic" false)
  (`KismetSystemLibrary.PrintString` "i collided and such")
  (`ActorComponent.Activate` (`self.shield_texture`) false)
  (`SceneComponent.SetHiddenInGame` _shield_overlap false false))

(event `shield_deactivated`
  (bind _shield_overlap (`self.shield_overlap`))
  ;[1 1 1] Shield Logic
  (`PrimitiveComponent.SetCollisionProfileName` _shield_overlap "NoCollision" false)
  (`ActorComponent.Deactivate` (`self.shield_texture`))
  (`SceneComponent.SetHiddenInGame` _shield_overlap true true))

(fn `UserConstructionScript`)